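; LiveJson_BP is an actor that switches three spot lights on and off from live JSON data.
; On BeginPlay it starts a looping half-second timer that polls its JsonComp component through ReadFromJson.
; Each poll sets the visibility of SpotLightA, B and C from the matching LightA, LightB and LightC booleans, so changes in the data show up during play.
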(event Custom|CustomEvent
  (bind _data (Default|ReadfromJson (Variables|Default|GetJson_Comp)))
  (Utilities|FlowControl|Sequence
    (:then_0
      (Rendering|SetVisibility (Variables|Default|GetSpotLight%20A) (.lighta _data) false))
    (:then_1
      (Rendering|SetVisibility (Variables|Default|GetSpotLight%20B) (.lightb _data) false))
    (:then_2
      (Rendering|SetVisibility (Variables|Default|GetSpotLight%20%20C) (.lightc _data) false))))

(event EventBeginPlay
  (Utilities|Time|SetTimerbyEvent (delegate Custom|CustomEvent) 0.5 true))

(fn ConstructionScript)