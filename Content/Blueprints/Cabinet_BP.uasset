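; Clickable cabinet actor that shows its ID, temperature or weight on camera-facing text.
; The UI's report change event raises a sunken cabinet, updates the text and recolors material and lights by judged temperature or weight level, or default for name.
; Clicking sends data to the UI, has CabinetManager_BP sink the others, then blends to and possesses its child Cabinet_Pawn.
; A reversible Timeline drives the vertical dive.
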(event OnClicked(CabinetMesh)
  (params (TouchedComponent :type Primitive%20Component%20Object%20Reference) (ButtonPressed :type Key%20Structure :default "None"))
  (bind _spectator_pawn (Variables|Default|GetSpectator%20Pawn))
  (bind _childactor (Variables|/Script/Engine.ChildActorComponent|GetChildActor _spectator_pawn))
  (bind _ascabinet_pawn (Utilities|Casting|CastToCabinet_Pawn _childactor))
  ;[1 1 1] On Clicked
  (Default|UpdateDetails (Variables|Default|GetMain%20UI%20Ref) (Variables|Default|GetCabinetData))
  (bind _returnvalue (Actor|GetActorOfClass "/Game/Blueprints/CabinetManager_BP.CabinetManager_BP_C"))
  (Default|AnimateCabinates _returnvalue true (.id (Variables|Default|GetCabinetData)))
  (Utilities|FlowControl|Sequence
    (:then_0
      (if (Variables|Default|GetisDived?\)
        (CallFunction|AnimateCabinate false)))
    (:then_1
      (bind _asmain_playercontroller (Utilities|Casting|CastToMain_Playercontroller (Game|GetPlayerController 0)))
      (Game|Player|SetViewTargetwithBlend _asmain_playercontroller _ascabinet_pawn 1.0 "VTBlend_Linear" 0.0 false)
      (Utilities|FlowControl|Delay 1.0)
      (Pawn|Possess _asmain_playercontroller _ascabinet_pawn))))

(event Custom|ChangeReport
  (params (Report%20Type :type E_ReportType%20Enum :default "NewEnumerator0"))
  (bind _cabinetdata (Variables|Default|GetCabinetData))
  (bind _cabinetdata_2 (Variables|Default|GetCabinetData))
  ;[1 1 1] Change Report
  (Utilities|FlowControl|Sequence
    (:then_0
      (if (Variables|Default|GetisDived?\)
        (CallFunction|AnimateCabinate false)))
    (:then_1
      (Rendering|Components|TextRender|SetText (Variables|Default|GetTextRender) (Utilities|Select :Index Report%20Type :NewEnumerator0 (Utilities|Text|FormatText "{0}" (.id _cabinetdata)) :NewEnumerator1 (Utilities|Text|FormatText "{0} °C" (.tempreture _cabinetdata)) :NewEnumerator2 (Utilities|Text|FormatText "{0} Kg" (.weight _cabinetdata))))
      (switch Utilities|FlowControl|Switch|SwitchonE_ReportType Report%20Type
        (:NewEnumerator0
          (CallFunction|ChangeAttire "NewEnumerator3"))
        (:NewEnumerator1
          (CallFunction|ChangeAttire (CallFunction|JudgeTemp (.tempreture _cabinetdata_2))))
        (:NewEnumerator2
          (CallFunction|ChangeAttire (CallFunction|JudgeWeight (.weight _cabinetdata_2))))))))

(event Custom|Change%20Attire
  (params (Scalar :type E_MeasureScalar%20Enum :default "NewEnumerator0"))
  (bind _cabinet_mesh (Variables|Default|GetCabinet%20Mesh))
  ;[1 1 1] Change Color
  (switch Utilities|FlowControl|Switch|SwitchonE_MeasureScalar Scalar
    (:NewEnumerator3
      (Rendering|Material|SetMaterial _cabinet_mesh 0 "/Game/Assets/Materials/Dev_DefaultCabinet_Inst2.Dev_DefaultCabinet_Inst2")
      (Rendering|Components|Light|SetLightColor (Variables|Default|GetSpotLight) "(R=1.000000,G=1.000000,B=1.000000,A=1.000000)" true))
    (:NewEnumerator0
      (Rendering|Material|SetMaterial _cabinet_mesh 0 "/Game/Assets/Materials/Dev_HighCabinet_Inst2.Dev_HighCabinet_Inst2")
      (Rendering|Components|Light|SetLightColor (Variables|Default|GetSpotLight) "(R=1.000000,G=0.000000,B=0.000000,A=1.000000)" true))
    (:NewEnumerator1
      (Rendering|Material|SetMaterial _cabinet_mesh 0 "/Game/Assets/Materials/Dev_MidCabinet_Inst1.Dev_MidCabinet_Inst1")
      (Rendering|Components|Light|SetLightColor (Variables|Default|GetSpotLight) "(R=1.000000,G=1.000000,B=0.000000,A=1.000000)" true))
    (:NewEnumerator2
      (Rendering|Material|SetMaterial _cabinet_mesh 0 "/Game/Assets/Materials/Dev_LowCabinet_Inst.Dev_LowCabinet_Inst")
      (Rendering|Components|Light|SetLightColor (Variables|Default|GetSpotLight) "(R=0.000000,G=1.000000,B=0.000000,A=1.000000)" true))))

(event Custom|Animate%20Cabinate
  (params (Dive? :type Boolean))
  (bind _cabinet_mesh (Variables|Default|GetCabinet%20Mesh))
  (bind _relativelocation (Variables|/Script/Engine.SceneComponent|GetRelativeLocation _cabinet_mesh))
  ;[1 1 1] Animate Cabinet
  (if (not (== (Variables|Default|GetisDived?\) Dive?))
    (Variables|Default|SetisDived?\ Dive?)
    (if Dive?
      (bind _newtrack_0 (Timeline|Timeline PlayFromStart)
        (:Update
          (Transformation|SetRelativeLocation _cabinet_mesh (Math|Vector|MakeVector (.x _relativelocation) (.y _relativelocation) (Math|Float|Lerp 1e+02 -1e+02 _newtrack_0)) false false)))
      (else
        (Timeline|Timeline ReverseFromEnd)))))

(event EventTick
  (params (DeltaSeconds :type Float%20%28single-precision%29))
  (Transformation|SetWorldRotation (Variables|Default|GetTextRender) (Math|Rotator|FindLookatRotation (Transformation|GetWorldLocation (Variables|Default|GetTextRender)) (Transformation|GetWorldLocation (Variables|/Script/Engine.PlayerCameraManager|GetTransformComponent (Game|GetPlayerCameraManager 0)))) false false))

(event EventBeginPlay
  (Rendering|Components|TextRender|SetText (Variables|Default|GetTextRender) (Utilities|Text|ToText(String) (.id (Variables|Default|GetCabinetData))))
  (Utilities|FlowControl|Delay 1.0)
  (bind _asmain_playercontroller (Utilities|Casting|CastToMain_Playercontroller (Game|GetPlayerController 0)))
  (Variables|Default|SetMain%20UI%20Ref (Variables|/Game/Blueprints/Main_Playercontroller.Main_Playercontroller_C|GetMain%20UI%20Ref _asmain_playercontroller))
  (EventDispatchers|BindEventtoChangeReport (Variables|/Game/Blueprints/Main_Playercontroller.Main_Playercontroller_C|GetMain%20UI%20Ref _asmain_playercontroller) (EventDispatchers|CreateEvent :!event Custom|ChangeReport)))

(fn ConstructionScript)