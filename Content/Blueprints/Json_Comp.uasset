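; Json component that loads on/off states for three lights (A, B, C) from a JSON file.
; ReadFromJson opens the file at JsonPath, copies each light field into the FileData struct in sequence, then returns that struct.
; The writetojsonfile event and BeginPlay are empty; the string-to-JSON and save-to-file nodes in the event graph are unconnected, so nothing is written.
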(event Custom|write%20to%20json%20file
  (params (Struct :type F%20Json%20Data%20Structure) (Path :type String)))

(event EventBeginPlay)

(fn ReadfromJson
  (bind _outjsonobject (Class|JsonBlueprintFunctionLibrary|FromFile (Utilities|Struct|MakeFilePath (Variables|Default|GetJson%20Path))))
  (Utilities|FlowControl|Sequence
    (:then_0
      (bind _outvalue (|GetJsonField _outjsonobject "lightA"))
      (Variables|Default|SetFile%20Data (Utilities|Struct|MakeF_JsonData (Class|KismetSystemLibrary|MakeLiteralBool _outvalue) (.lightb (Variables|Default|GetFile%20Data)) (.lightc (Variables|Default|GetFile%20Data)))))
    (:then_1
      (bind _outvalue_2 (|GetJsonField _outjsonobject "lightB"))
      (Variables|Default|SetFile%20Data (Utilities|Struct|MakeF_JsonData (.lighta (Variables|Default|GetFile%20Data)) (Class|KismetSystemLibrary|MakeLiteralBool _outvalue_2) (.lightc (Variables|Default|GetFile%20Data)))))
    (:then_2
      (bind _outvalue_3 (|GetJsonField _outjsonobject "lightC"))
      (Variables|Default|SetFile%20Data (Utilities|Struct|MakeF_JsonData (.lighta (Variables|Default|GetFile%20Data)) (.lightb (Variables|Default|GetFile%20Data)) (Class|KismetSystemLibrary|MakeLiteralBool _outvalue_3))))
    (:then_3
      (return (Variables|Default|GetFile%20Data)))))